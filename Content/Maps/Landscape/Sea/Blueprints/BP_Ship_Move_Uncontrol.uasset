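; Uncontrolled ship actor that sails automatically along a spline on a referenced ship path actor in the sea level.
; On BeginPlay, if the ship is active, it plays a timeline with a play rate set from the travel duration.
; Each update maps the timeline alpha to a distance along the spline and sets the actor's world location and rotation to that point.
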(event `self.ReceiveBeginPlay`
  ;[1 1 1] Активация объекта
  (if (`self.Active Ship`)
    (`self.Move Ship`)))

(event `Move Ship`
  (bind _shippath_2_spline (`/Game/Maps/Landscape/Sea/Blueprints/BP_Ship_Path_Uncontrol.ShipPath_2_Spline` (`self.ShipPathRef`)))
  (bind _returnvalue (`KismetMathLibrary.Lerp` 0.0 (`SplineComponent.GetSplineLength` _shippath_2_spline) (`self.Alpha`)))
  ;[1 1 1] Движение для одного объекта
  ;;[1 1 1] Установка скорости объекта
  (`TimelineComponent.SetPlayRate` (`self.TimePath`) (/ 1.0 (`self.Duration`)))
  ;;[1 1 1] Задать значение временной шкалы
  (bind (_direction _alpha) (`Timeline|TimePath`)
    (:`Update`
      (set `self.Alpha` _alpha)
      (`self.K2_SetActorLocationAndRotation` (`SplineComponent.GetLocationAtDistanceAlongSpline` _shippath_2_spline _returnvalue "World") (`SplineComponent.GetRotationAtDistanceAlongSpline` _shippath_2_spline _returnvalue "World")))))

(fn `UserConstructionScript`)
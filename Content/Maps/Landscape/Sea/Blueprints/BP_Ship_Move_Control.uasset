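; BP_Ship_Move_Control is a ship actor that the player starts and stops with the Interact input to travel along a spline path.
; Overlap of the ALS character with its Box enables input and opens a gate; leaving neither closes the gate nor disables input.
; Each press flip-flops between playing and stopping a timeline whose rate derives from Duration.
; The timeline alpha maps to distance along ShipPathRef's spline, setting world location and rotation.
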(event `InputAction|Interact`
  (params (Key :type "Key Structure"))
  ;[1 1 1] Активация/деактивация движения объекта
  (:`Pressed`
    (`/Engine/EditorBlueprintResources/StandardMacros.Gate` true :!label _label
      (:`Exit`
        (`/Engine/EditorBlueprintResources/StandardMacros.FlipFlop`
          (:`A`
            (`self.Move Ship`))
          (:`B`
            (`self.StopShip`)))))))

(event `self.Box.OnComponentBeginOverlap`
  (params (OverlappedComponent :type "PrimitiveComponent Object Reference") (OtherActor :type "Actor Object Reference") (OtherComp :type "PrimitiveComponent Object Reference") (OtherBodyIndex :type Integer) (bFromSweep :type Boolean) (SweepResult :type "HitResult Structure (by ref)"))
  ;[1 1 1] Активация/деактивация движения объекта
  (cast `/Game/AdvancedLocomotionV4/Blueprints/CharacterLogic/ALS_AnimMan_CharacterBP` OtherActor)
  (`self.EnableInput` (`GameplayStatics.GetPlayerController` 0))
  (goto _label :!via `Open`))

(event `self.Box.OnComponentEndOverlap`
  (params (OverlappedComponent :type "PrimitiveComponent Object Reference") (OtherActor :type "Actor Object Reference") (OtherComp :type "PrimitiveComponent Object Reference") (OtherBodyIndex :type Integer))
  ;[1 1 1] Активация/деактивация движения объекта
  (cast `/Game/AdvancedLocomotionV4/Blueprints/CharacterLogic/ALS_AnimMan_CharacterBP` OtherActor))

(event `Move Ship`
  (bind _shippathspline_unmove (`/Game/Maps/Landscape/Sea/Blueprints/BP_Ship_Path_Control.ShipPathSpline_Unmove` (`self.ShipPathRef`)))
  (bind _returnvalue (`KismetMathLibrary.Lerp` 0.0 (`SplineComponent.GetSplineLength` _shippathspline_unmove) (`self.Alpha`)))
  ;[1 1 1] Движение для одного объекта
  ;;[1 1 1] Установка скорости объекта
  (`TimelineComponent.SetPlayRate` (`self.TimePath`) (/ 1.0 (`self.Duration`)))
  ;;[1 1 1] Задать значение временной шкалы
  (bind (_direction _alpha) (`Timeline|TimePath` :!label _label_2)
    (:`Update`
      (set `self.Alpha` _alpha)
      (`self.K2_SetActorLocationAndRotation` (`SplineComponent.GetLocationAtDistanceAlongSpline` _shippathspline_unmove _returnvalue "World") (`SplineComponent.GetRotationAtDistanceAlongSpline` _shippathspline_unmove _returnvalue "World")))))

(event `StopShip`
  ;[1 1 1] Движение для одного объекта
  (goto _label_2 :!via `Stop`))

(fn `UserConstructionScript`)
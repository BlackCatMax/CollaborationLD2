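; Ship actor for the sea port that moves its static mesh along a scripted path from BeginPlay.
; A timeline drives two nested vector lerps on the mesh's relative location, travelling along negative Y, then blending toward an endpoint also offset in X.
; A box trigger enables the actor's input for player 0 while an ALS character overlaps it, though the graph defines no input events.
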(event `self.ReceiveBeginPlay`
  (bind (_direction _move_y _move_y_x) (`Timeline|Timeline_0`)
    (:`Update`
      (`SceneComponent.K2_SetRelativeLocation` (`self.StaticMesh`) (`KismetMathLibrary.VLerp` (`KismetMathLibrary.VLerp` (0.0 0.0 0.0) (-0.0 -11150.0 0.0) _move_y) (-2100.0 -22300.0 0.0) _move_y_x) false false))))

(event `self.Box.OnComponentBeginOverlap`
  (params (OverlappedComponent :type "PrimitiveComponent Object Reference") (OtherActor :type "Actor Object Reference") (OtherComp :type "PrimitiveComponent Object Reference") (OtherBodyIndex :type Integer) (bFromSweep :type Boolean) (SweepResult :type "HitResult Structure (by ref)"))
  (cast `/Game/AdvancedLocomotionV4/Blueprints/CharacterLogic/ALS_AnimMan_CharacterBP` OtherActor)
  (`self.EnableInput` (`GameplayStatics.GetPlayerController` 0)))

(event `self.Box.OnComponentEndOverlap`
  (params (OverlappedComponent :type "PrimitiveComponent Object Reference") (OtherActor :type "Actor Object Reference") (OtherComp :type "PrimitiveComponent Object Reference") (OtherBodyIndex :type Integer))
  (cast `/Game/AdvancedLocomotionV4/Blueprints/CharacterLogic/ALS_AnimMan_CharacterBP` OtherActor)
  (`self.DisableInput` (`GameplayStatics.GetPlayerController` 0)))

(fn `UserConstructionScript`)
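; Spline placement actor that fills its spline with copies of a chosen static mesh through a hierarchical instanced static mesh component.
; The construction script spaces instances by the mesh's X bounds times actor X scale, placing each by location only, without following spline rotation.
; A color scheme enum picks a material from an array, but the steps applying it, including a randomized dynamic-material variant, are disconnected.
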(fn `SwitchColorScheme`
  (params (Selection :type Byte :default 0))
  (returns (ReturnedMaterial :type "MaterialInstance Object Reference"))
  (locals (MyMaterial :type "MaterialInstance Object Reference"))
  (switch `|SwitchEnum` Selection
    (:`NewEnumerator0`
      (set `local.MyMaterial` (`|GetArrayItem` (`self.MaterialArray`))))
    (:`NewEnumerator1`
      (set `local.MyMaterial` (`|GetArrayItem` (`self.MaterialArray`) 1)))
    (:`NewEnumerator2`
      (set `local.MyMaterial` (`|GetArrayItem` (`self.MaterialArray`) 2)))
    (:`NewEnumerator3`
      (set `local.MyMaterial` (`|GetArrayItem` (`self.MaterialArray`) 3)))
    (:`NewEnumerator4`
      (set `local.MyMaterial` (`|GetArrayItem` (`self.MaterialArray`) 4)))
    (:`NewEnumerator8`
      (set `local.MyMaterial` (`|GetArrayItem` (`self.MaterialArray`) 5))))
  (return (`local.MyMaterial`)))

(fn `UserConstructionScript`
  (bind _returnvalue_x (`KismetMathLibrary.BreakVector` (`self.GetActorScale3D`)))
  (bind (_min _max) (break `Box` (`StaticMesh.GetBoundingBox` (`self.MyStaticMesh`))))
  ;[0 1 0.6953] Defines a section length and the static mesh
  (`StaticMeshComponent.SetStaticMesh` (`self.HierarchicalInstancedStaticMesh`) (`self.MyStaticMesh`)) ; Public Var, individual to each actors
  (set `self.SectionLengthCoef` (- (.x _max) (.x _min)))
  (set `self.SectionLength` (* _returnvalue_x (`self.SectionLengthCoef`)))
  ;[0.3828 1 0] For each sections based on the length of the spline divided by the defined section length, add an instance of the static mesh at the desired location following the index times the section length
  (for _index (range (`KismetMathLibrary.FTrunc` (/ (`SplineComponent.GetSplineLength` (`self.Spline`)) (`self.SectionLength`))))
    (set `self.Current Index` _index)
    (bind _returnvalue (`InstancedStaticMeshComponent.AddInstance` (`self.HierarchicalInstancedStaticMesh`) (`KismetMathLibrary.Conv_VectorToTransform` (`SplineComponent.GetLocationAtDistanceAlongSpline` (`self.Spline`) (* (`self.Current Index`) (`self.SectionLength`)) "Local")) false))
    ;;[0 0.1562 1] Color Scheme Function
    (bind _returnedmaterial (`self.SwitchColorScheme` (`self.ColorScheme`)))))
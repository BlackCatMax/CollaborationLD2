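; BP_Gears is a gear pickup that the ALS AnimMan character collects by pressing Interact.
; The construction script applies the chosen mesh, and sphere overlap toggles input and a gate so pickup works only in range.
; Pickup requires an empty HasGear flag, sets it, matches the mesh name (Simple, Corner, Helix) to an overlay state, then destroys its components.
; An unmatched name loops back into the checks endlessly.
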(event `InputAction|Interact`
  (params (Key :type "Key Structure"))
  (bind _returnvalue (`KismetSystemLibrary.GetObjectName` (`self.New Mesh`)))
  (:`Pressed`
    (if (not (`/Game/AdvancedLocomotionV4/Blueprints/CharacterLogic/ALS_AnimMan_CharacterBP.HasGear?` (stale `self.Sphere.OnComponentBeginOverlap` _asals_anim_man_character_bp)))
      (`/Engine/EditorBlueprintResources/StandardMacros.Gate` true :!label _label
        (:`Exit`
          (set `/Game/AdvancedLocomotionV4/Blueprints/CharacterLogic/ALS_AnimMan_CharacterBP.HasGear?` true (stale `self.Sphere.OnComponentBeginOverlap` _asals_anim_man_character_bp))
          (if (`KismetStringLibrary.Contains` _returnvalue "Simple") :!label _label_2
            (`/Game/AdvancedLocomotionV4/Blueprints/Interfaces/ALS_Character_BPI.BPI_Set_OverlayState` (stale `self.Sphere.OnComponentBeginOverlap` _asals_anim_man_character_bp) "NewEnumerator8")
            (elif (`KismetStringLibrary.Contains` _returnvalue "Corner")
              (`/Game/AdvancedLocomotionV4/Blueprints/Interfaces/ALS_Character_BPI.BPI_Set_OverlayState` (stale `self.Sphere.OnComponentBeginOverlap` _asals_anim_man_character_bp) "NewEnumerator9")
              (elif (`KismetStringLibrary.Contains` _returnvalue "Helix")
                (`/Game/AdvancedLocomotionV4/Blueprints/Interfaces/ALS_Character_BPI.BPI_Set_OverlayState` (stale `self.Sphere.OnComponentBeginOverlap` _asals_anim_man_character_bp) "NewEnumerator11")
                (else
                  (goto _label_2)))))
          (`ActorComponent.K2_DestroyComponent` (`self.StaticMesh`))
          (`ActorComponent.K2_DestroyComponent` (`self.Sphere`))
          (`ActorComponent.K2_DestroyComponent` (`self.DefaultSceneRoot`))
          (`KismetSystemLibrary.PrintString` "GEAR FOUND" true true (struct :`G` 1.0 :`A` 1.0) 5.0))))))

(event `self.Sphere.OnComponentBeginOverlap`
  (params (OverlappedComponent :type "PrimitiveComponent Object Reference") (OtherActor :type "Actor Object Reference") (OtherComp :type "PrimitiveComponent Object Reference") (OtherBodyIndex :type Integer) (bFromSweep :type Boolean) (SweepResult :type "HitResult Structure (by ref)"))
  (bind _asals_anim_man_character_bp (cast `/Game/AdvancedLocomotionV4/Blueprints/CharacterLogic/ALS_AnimMan_CharacterBP` OtherActor))
  (`self.EnableInput` (`GameplayStatics.GetPlayerController` 0))
  (goto _label :!via `Open`))

(event `self.Sphere.OnComponentEndOverlap`
  (params (OverlappedComponent :type "PrimitiveComponent Object Reference") (OtherActor :type "Actor Object Reference") (OtherComp :type "PrimitiveComponent Object Reference") (OtherBodyIndex :type Integer))
  (cast `/Game/AdvancedLocomotionV4/Blueprints/CharacterLogic/ALS_AnimMan_CharacterBP` OtherActor)
  (`self.DisableInput` (`GameplayStatics.GetPlayerController` 0) :!label _label_3)
  (goto _label :!via `Close`))

(event `self.ReceiveBeginPlay`
  (goto _label_3))

(fn `UserConstructionScript`
  (`StaticMeshComponent.SetStaticMesh` (`self.StaticMesh`) (`self.New Mesh`)))
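; BP_TestRail is a test rail actor that slides a motor along a track while a linked Panel's EventON flag is set.
; Every Tick plays the MoveRail timeline at the Speed rate when the flag is on, or reverses it when off.
; The timeline's Alpha lerps the Motor between start and end locations and spins two rollers through two full yaw turns in sync.
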(event `self.ReceiveTick`
  (params (DeltaSeconds :type "Float (single-precision)"))
  (if (`/Game/Blueprints/BP_RepairSystem.EventON` (`self.Panel`))
    (`TimelineComponent.SetPlayRate` (`self.MoveRail`) (`self.Speed`))
    (bind (_direction _alpha) (`Timeline|MoveRail` :!label _label)
      (:`Update`
        (`SceneComponent.K2_SetRelativeLocation` (`self.Motor`) (`KismetMathLibrary.VLerp` (`self.StartLocation`) (`self.EndLocation`) _alpha) false false)
        (`SceneComponent.K2_SetRelativeRotation` (`self.SM_Roller_D_01`) (`KismetMathLibrary.MakeRotator` 0.0 0.0 (`KismetMathLibrary.Lerp` 0.0 -720.0 _alpha)) false false)
        (`SceneComponent.K2_SetRelativeRotation` (`self.SM_Roller_D_02`) (`KismetMathLibrary.MakeRotator` 0.0 0.0 (`KismetMathLibrary.Lerp` 0.0 -720.0 _alpha)) false false)))
    (else
      (goto _label :!via `Reverse`))))

(fn `UserConstructionScript`)
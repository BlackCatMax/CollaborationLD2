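; BP_Chest is an interactable chest that can require a key before it opens.
; Overlapping its sphere caches the ALS AnimMan character and enables input, which is disabled on exit and at BeginPlay.
; Interact plays a timeline that moves and rolls the lid mesh, consuming the key on first unlock, or prints a warning without one.
; Once no key is needed, a FlipFlop alternates opening and closing.
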(event `InputAction|Interact`
  (params (Key :type "Key Structure"))
  (:`Pressed`
    (if (`self.Need Key?`)
      (if (`/Game/AdvancedLocomotionV4/Blueprints/CharacterLogic/ALS_AnimMan_CharacterBP.HasKey?` (stale `self.Sphere.OnComponentBeginOverlap` _asals_anim_man_character_bp))
        (`|ExecutionSequence`
          (:`then_0`
            (bind (_direction _open_close) (`Timeline|Open-Close` :`NewTime` 0.1 :!label _label)
              (:`Update`
                (`SceneComponent.K2_SetRelativeLocationAndRotation` (`self.SM_Chest_PartB`) (65.0 -32.0 60.0) (`KismetMathLibrary.MakeRotator` _open_close) false false))))
          (:`then_1`
            (`/Engine/EditorBlueprintResources/StandardMacros.DoOnce` false
              (:`Completed`
                (set `self.Need Key?` false)
                (set `/Game/AdvancedLocomotionV4/Blueprints/CharacterLogic/ALS_AnimMan_CharacterBP.HasKey?` false (stale `self.Sphere.OnComponentBeginOverlap` _asals_anim_man_character_bp))))))
        (else
          (`KismetSystemLibrary.PrintString` "I NEED A KEY" true true (struct :`R` 1.0 :`A` 1.0) 5.0)))
      (else
        (`/Engine/EditorBlueprintResources/StandardMacros.FlipFlop`
          (:`A`
            (goto _label))
          (:`B`
            (goto _label :!via `Reverse`)))))))

(event `self.Sphere.OnComponentBeginOverlap`
  (params (OverlappedComponent :type "PrimitiveComponent Object Reference") (OtherActor :type "Actor Object Reference") (OtherComp :type "PrimitiveComponent Object Reference") (OtherBodyIndex :type Integer) (bFromSweep :type Boolean) (SweepResult :type "HitResult Structure (by ref)"))
  (bind _asals_anim_man_character_bp (cast `/Game/AdvancedLocomotionV4/Blueprints/CharacterLogic/ALS_AnimMan_CharacterBP` OtherActor))
  (`self.EnableInput` (`GameplayStatics.GetPlayerController` 0)))

(event `self.Sphere.OnComponentEndOverlap`
  (params (OverlappedComponent :type "PrimitiveComponent Object Reference") (OtherActor :type "Actor Object Reference") (OtherComp :type "PrimitiveComponent Object Reference") (OtherBodyIndex :type Integer))
  (cast `/Game/AdvancedLocomotionV4/Blueprints/CharacterLogic/ALS_AnimMan_CharacterBP` OtherActor)
  (`self.DisableInput` (`GameplayStatics.GetPlayerController` 0) :!label _label_2))

(event `self.ReceiveBeginPlay`
  (goto _label_2))

(fn `UserConstructionScript`)
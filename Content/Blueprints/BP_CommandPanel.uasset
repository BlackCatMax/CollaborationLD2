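; BP_CommandPanel is a configurable panel with five indicator lamps showing repair flags for mechanism parts like gears, worm and pulley.
; Construction sets its mesh, scale and trigger box.
; BeginPlay snaps lamps to sockets and creates dynamic emissive materials: red with Speed set when a flag is true, otherwise green; the fifth has no flag.
; Player overlap toggles input and a gate, which starts closed, though nothing shown runs through it.
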(event `InputAction|Interact`
  (params (Key :type "Key Structure")))

(event `self.BoxMech.OnComponentBeginOverlap`
  (params (OverlappedComponent :type "PrimitiveComponent Object Reference") (OtherActor :type "Actor Object Reference") (OtherComp :type "PrimitiveComponent Object Reference") (OtherBodyIndex :type Integer) (bFromSweep :type Boolean) (SweepResult :type "HitResult Structure (by ref)"))
  (cast `/Game/AdvancedLocomotionV4/Blueprints/CharacterLogic/ALS_AnimMan_CharacterBP` OtherActor)
  (`self.EnableInput` (`GameplayStatics.GetPlayerController` 0))
  (`/Engine/EditorBlueprintResources/StandardMacros.Gate` true :!via `Open` :!label _label))

(event `self.BoxMech.OnComponentEndOverlap`
  (params (OverlappedComponent :type "PrimitiveComponent Object Reference") (OtherActor :type "Actor Object Reference") (OtherComp :type "PrimitiveComponent Object Reference") (OtherBodyIndex :type Integer))
  (cast `/Game/AdvancedLocomotionV4/Blueprints/CharacterLogic/ALS_AnimMan_CharacterBP` OtherActor)
  (`self.DisableInput` (`GameplayStatics.GetPlayerController` 0) :!label _label_2)
  (goto _label :!via `Close`))

(event `self.ReceiveBeginPlay`
  (bind _lamp05 (`self.Lamp05`))
  (bind _lamp01 (`self.Lamp01`))
  (bind _lamp02 (`self.Lamp02`))
  (bind _lamp03 (`self.Lamp03`))
  (bind _lamp04 (`self.Lamp04`))
  (`|ExecutionSequence`
    (:`then_0`
      (goto _label_2))
    (:`then_1`
      (`self.LampSettings` _lamp01 _lamp01 (`self.BigGearRepaired`) "Lamp01"))
    (:`then_2`
      (`self.LampSettings` _lamp02 _lamp02 (`self.ConeGearRepaired`) "Lamp02"))
    (:`then_3`
      (`self.LampSettings` _lamp03 _lamp03 (`self.WormRepaired`) "Lamp03"))
    (:`then_4`
      (`self.LampSettings` _lamp04 _lamp04 (`self.PulleyRepaired`) "Lamp04"))
    (:`then_5`
      (`self.LampSettings` _lamp05 _lamp05 false "Lamp05"))))

(fn `LampSettings`
  (params (LampMesh01 :type "SceneComponent Object Reference") (LampMesh02 :type "PrimitiveComponent Object Reference") (RepairedDetail :type Boolean) (InSocketName :type Name))
  (bind (_returnvalue_location _returnvalue_rotation _returnvalue_scale) (`KismetMathLibrary.BreakTransform` (`SceneComponent.GetSocketTransform` (`self.BasePanel`) InSocketName "RTS_World")))
  (`SceneComponent.K2_SetWorldTransform` LampMesh01 (`KismetMathLibrary.MakeTransform` _returnvalue_location _returnvalue_rotation _returnvalue_scale) false false)
  (if RepairedDetail
    (bind _returnvalue (`PrimitiveComponent.CreateDynamicMaterialInstance` LampMesh02 0 "/Game/Materials/MI_DetailsEmissive_Orange.MI_DetailsEmissive_Orange" "None"))
    (`MaterialInstanceDynamic.SetVectorParameterValue` _returnvalue "EmissiveColor" (struct :`R` 0.5 :`A` 1.0))
    (`MaterialInstanceDynamic.SetScalarParameterValue` _returnvalue "EmissivePower" 40.0)
    (`MaterialInstanceDynamic.SetScalarParameterValue` _returnvalue "Speed" 1.0)
    (else
      (bind _returnvalue_2 (`PrimitiveComponent.CreateDynamicMaterialInstance` LampMesh02 0 "/Game/Materials/MI_DetailsEmissive_Orange.MI_DetailsEmissive_Orange" "None"))
      (`MaterialInstanceDynamic.SetVectorParameterValue` _returnvalue_2 "EmissiveColor" (struct :`G` 0.5 :`A` 1.0))
      (`MaterialInstanceDynamic.SetScalarParameterValue` _returnvalue_2 "EmissivePower" 20.0))))

(fn `UserConstructionScript`
  (bind _basepanel (`self.BasePanel`))
  (bind _scale (`self.Scale`))
  (set `PrimitiveComponent.bGenerateOverlapEvents` (`self.Generate Overlap Events`) (`self.BoxMech`))
  (`SceneComponent.SetWorldScale3D` _basepanel (`KismetMathLibrary.MakeVector` _scale _scale _scale))
  (`StaticMeshComponent.SetStaticMesh` _basepanel (`self.TargetBase`))
  (`SceneComponent.K2_SetRelativeTransform` (`self.BoxMech`) (`self.BoxCollisionTransform`) false false))
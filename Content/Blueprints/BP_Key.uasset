(event `InputAction|Interact`
  (params (Key :type "Key Structure"))
  (bind _keystypes (`self.KeysTypes`))
  (:`Pressed`
    (`/Engine/EditorBlueprintResources/StandardMacros.Gate` true :!label _label
      (:`Exit`
        (`KismetArrayLibrary.Array_Add` (`/Game/AdvancedLocomotionV4/Blueprints/CharacterLogic/ALS_AnimMan_CharacterBP.OwnedKeys` (stale `self.Sphere.OnComponentBeginOverlap` _asals_anim_man_character_bp)) _keystypes)
        (`|ExecutionSequence`
          (:`then_0`
            (bind _returnvalue (`|CreateWidget` "/Game/UI/WB_YouFound.WB_YouFound_C"))
            (`UserWidget.AddToViewport` _returnvalue 0))
          (:`then_1`
            (bind _returnvalue_2 (`|CreateWidget` (select `/Game/Blueprints/ENUM/KeysTypes` _keystypes :`NewEnumerator0` "/Game/UI/WB_IronKey_Chest.WB_IronKey_Chest_C" :`NewEnumerator1` "/Game/UI/WB_SilverKey_Chest.WB_SilverKey_Chest_C" :`NewEnumerator2` "/Game/UI/WB_GoldKey_Chest.WB_GoldKey_Chest_C" :`NewEnumerator3` "/Game/UI/WB_IronKey_Door.WB_IronKey_Door_C" :`NewEnumerator4` "/Game/UI/WB_SilverKey_Door.WB_SilverKey_Door_C" :`NewEnumerator5` "/Game/UI/WB_GoldKey_Door.WB_GoldKey_Door_C" :!type "UserWidget Class Reference")))
            (`UserWidget.AddToViewport` _returnvalue_2 0)
            (`self.K2_DestroyActor`)))))))

(event `self.Sphere.OnComponentBeginOverlap`
  (params (OverlappedComponent :type "PrimitiveComponent Object Reference") (OtherActor :type "Actor Object Reference") (OtherComp :type "PrimitiveComponent Object Reference") (OtherBodyIndex :type Integer) (bFromSweep :type Boolean) (SweepResult :type "HitResult Structure (by ref)"))
  (bind _asals_anim_man_character_bp (cast `/Game/AdvancedLocomotionV4/Blueprints/CharacterLogic/ALS_AnimMan_CharacterBP` OtherActor))
  (`self.EnableInput` (`GameplayStatics.GetPlayerController` 0))
  (goto _label :!via `Open`))

(event `self.Sphere.OnComponentEndOverlap`
  (params (OverlappedComponent :type "PrimitiveComponent Object Reference") (OtherActor :type "Actor Object Reference") (OtherComp :type "PrimitiveComponent Object Reference") (OtherBodyIndex :type Integer))
  (cast `/Game/AdvancedLocomotionV4/Blueprints/CharacterLogic/ALS_AnimMan_CharacterBP` OtherActor)
  (`self.DisableInput` (`GameplayStatics.GetPlayerController` 0) :!label _label_2)
  (goto _label :!via `Close`))

(event `self.ReceiveBeginPlay`
  (goto _label_2))

(fn `UserConstructionScript`
  (bind _returnvalue (`PrimitiveComponent.CreateDynamicMaterialInstance` (`self.SM_Key`) 0 "/Game/Materials/MI_Details.MI_Details" "None"))
  (`MaterialInstanceDynamic.SetVectorParameterValue` _returnvalue "Color" (select `/Game/Blueprints/ENUM/KeysTypes` (`self.KeysTypes`) :`NewEnumerator0` (struct :`R` 0.1 :`G` 0.1 :`B` 0.1 :`A` 1.0) :`NewEnumerator1` (struct :`R` 0.5 :`G` 0.5 :`B` 0.5 :`A` 1.0) :`NewEnumerator2` (struct :`R` 1.0 :`G` 0.5 :`A` 1.0) :`NewEnumerator3` (struct :`R` 0.1 :`G` 0.1 :`B` 0.1 :`A` 1.0) :`NewEnumerator4` (struct :`R` 0.5 :`G` 0.5 :`B` 0.5 :`A` 1.0) :`NewEnumerator5` (struct :`R` 1.0 :`G` 0.5 :`A` 1.0) :!type "LinearColor Structure")))
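; Prototype elevator actor that lets the player pick one of three floors with the 1, 2 and 3 keys.
; Input turns on when a Pawn enters the Box trigger and is never disabled.
; A timeline samples the spline to drive the Elevator's Z, stopping once it reaches the selected floor's spline point height.
; The timeline only plays forward, with no logic for descending to lower floors.
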(event `Key|One`
  (params (Key :type "Key Structure"))
  (bind _spline (`self.Spline`))
  (bind (_returnvalue_x _returnvalue_y _returnvalue_z) (`KismetMathLibrary.BreakVector` (`SplineComponent.GetLocationAtSplinePoint` _spline (`self.Floor`) "Local")))
  (:`Pressed`
    (set `self.Floor` 0)
    (bind (_direction _newtrack_1) (`Timeline|Timeline_0` :!label _label)
      (:`Update`
        (bind (_returnvalue_x_2 _returnvalue_y_2 _returnvalue_z_2) (`KismetMathLibrary.BreakVector` (`SplineComponent.GetLocationAtTime` _spline _newtrack_1 "Local" false)))
        (if (< _returnvalue_z_2 _returnvalue_z)
          (`SceneComponent.K2_SetRelativeLocation` (`self.Elevator`) (`KismetMathLibrary.MakeVector` 0.0 0.0 _returnvalue_z_2) false false)
          (else
            (goto _label :!via `Stop`)))))))

(event `Key|Two`
  (params (Key :type "Key Structure"))
  (:`Pressed`
    (set `self.Floor` 1)
    (goto _label)))

(event `Key|Three`
  (params (Key :type "Key Structure"))
  (:`Pressed`
    (set `self.Floor` 2)
    (goto _label)))

(event `self.Box.OnComponentBeginOverlap`
  (params (OverlappedComponent :type "PrimitiveComponent Object Reference") (OtherActor :type "Actor Object Reference") (OtherComp :type "PrimitiveComponent Object Reference") (OtherBodyIndex :type Integer) (bFromSweep :type Boolean) (SweepResult :type "HitResult Structure (by ref)"))
  (cast `Pawn` OtherActor)
  (`self.EnableInput` (`GameplayStatics.GetPlayerController` 0)))

(fn `UserConstructionScript`)
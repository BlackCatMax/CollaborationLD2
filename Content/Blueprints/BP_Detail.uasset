(event `InputAction|Interact`
  (params (Key :type "Key Structure"))
  (bind _detailtypes (`self.DetailTypes`))
  (:`Pressed`
    (if (not (`/Game/AdvancedLocomotionV4/Blueprints/CharacterLogic/ALS_AnimMan_CharacterBP.PickUpDetail` (stale `self.Sphere.OnComponentBeginOverlap` _asals_anim_man_character_bp)))
      (`/Engine/EditorBlueprintResources/StandardMacros.Gate` true :!label _label
        (:`Exit`
          (set `/Game/AdvancedLocomotionV4/Blueprints/CharacterLogic/ALS_AnimMan_CharacterBP.PickUpDetail` true (stale `self.Sphere.OnComponentBeginOverlap` _asals_anim_man_character_bp))
          (if (`|EnumEquality` _detailtypes "NewEnumerator1")
            (`/Game/AdvancedLocomotionV4/Blueprints/Interfaces/ALS_Character_BPI.BPI_Set_OverlayState` (stale `self.Sphere.OnComponentBeginOverlap` _asals_anim_man_character_bp) "NewEnumerator8")
            (`|ExecutionSequence` :!label _label_2
              (:`then_0`
                (bind _returnvalue (`|CreateWidget` "/Game/UI/WB_YouFound.WB_YouFound_C"))
                (`UserWidget.AddToViewport` _returnvalue 0))
              (:`then_1`
                (bind _returnvalue_2 (`|CreateWidget` (select `/Game/Blueprints/DetailTypes` (`self.DetailTypes`) :`NewEnumerator0` "/Game/UI/WB_GearBig.WB_GearBig_C" :`NewEnumerator1` "/Game/UI/WB_GearCone.WB_GearCone_C" :`NewEnumerator2` "/Game/UI/WB_GearWorm.WB_GearWorm_C" :`NewEnumerator3` "/Game/UI/WB_Pulley.WB_Pulley_C" :!type "UserWidget Class Reference")))
                (`UserWidget.AddToViewport` _returnvalue_2 0)
                (`self.K2_DestroyActor`)))
            (elif (`|EnumEquality` _detailtypes "NewEnumerator0")
              (`/Game/AdvancedLocomotionV4/Blueprints/Interfaces/ALS_Character_BPI.BPI_Set_OverlayState` (stale `self.Sphere.OnComponentBeginOverlap` _asals_anim_man_character_bp) "NewEnumerator9")
              (goto _label_2)
              (elif (`|EnumEquality` _detailtypes "NewEnumerator2")
                (`/Game/AdvancedLocomotionV4/Blueprints/Interfaces/ALS_Character_BPI.BPI_Set_OverlayState` (stale `self.Sphere.OnComponentBeginOverlap` _asals_anim_man_character_bp) "NewEnumerator11")
                (goto _label_2)
                (elif (`|EnumEquality` _detailtypes "NewEnumerator3")
                  (`/Game/AdvancedLocomotionV4/Blueprints/Interfaces/ALS_Character_BPI.BPI_Set_OverlayState` (stale `self.Sphere.OnComponentBeginOverlap` _asals_anim_man_character_bp) "NewEnumerator7")
                  (goto _label_2))))))))))

(event `self.Sphere.OnComponentBeginOverlap`
  (params (OverlappedComponent :type "PrimitiveComponent Object Reference") (OtherActor :type "Actor Object Reference") (OtherComp :type "PrimitiveComponent Object Reference") (OtherBodyIndex :type Integer) (bFromSweep :type Boolean) (SweepResult :type "HitResult Structure (by ref)"))
  (bind _asals_anim_man_character_bp (cast `/Game/AdvancedLocomotionV4/Blueprints/CharacterLogic/ALS_AnimMan_CharacterBP` OtherActor))
  (`self.EnableInput` (`GameplayStatics.GetPlayerController` 0))
  (goto _label :!via `Open`))

(event `self.Sphere.OnComponentEndOverlap`
  (params (OverlappedComponent :type "PrimitiveComponent Object Reference") (OtherActor :type "Actor Object Reference") (OtherComp :type "PrimitiveComponent Object Reference") (OtherBodyIndex :type Integer))
  (cast `/Game/AdvancedLocomotionV4/Blueprints/CharacterLogic/ALS_AnimMan_CharacterBP` OtherActor)
  (`self.DisableInput` (`GameplayStatics.GetPlayerController` 0) :!label _label_3)
  (goto _label :!via `Close`))

(event `self.ReceiveBeginPlay`
  (goto _label_3))

(fn `UserConstructionScript`
  (`StaticMeshComponent.SetStaticMesh` (`self.DetailStaticMesh`) (select `/Game/Blueprints/DetailTypes` (`self.DetailTypes`) :`NewEnumerator0` "/Game/Meshes/Mechanics/SM_BigGear.SM_BigGear" :`NewEnumerator1` "/Game/Meshes/Mechanics/SM_ConeGear.SM_ConeGear" :`NewEnumerator2` "/Game/Meshes/Mechanics/SM_Worm.SM_Worm" :`NewEnumerator3` "/Game/Meshes/Mechanics/SM_PulleyGround.SM_PulleyGround" :!type "StaticMesh Object Reference"))
  (set `PrimitiveComponent.bGenerateOverlapEvents` (`self.Generate Overlap Events`) (`self.Sphere`)))
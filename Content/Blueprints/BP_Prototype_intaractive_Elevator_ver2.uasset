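; Prototype interactive elevator that travels vertically between three floors, each defined by a spline point.
; Overlapping the box with a pawn enables input, and number keys 1 to 3 set the target floor.
; The floor comparison plays or reverses a timeline at a set speed, sampling spline height to move the elevator.
; The timeline stops and records the current floor once that height reaches the target point.
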(event `Key|One`
  (params (Key :type "Key Structure"))
  (bind _spline (`self.Spline`))
  (bind _spline_2 (`self.Spline`))
  (bind _timeline_0 (`self.Timeline_0`))
  (bind _speed (`self.Speed`))
  (bind (_returnvalue_x _returnvalue_y _returnvalue_z) (`KismetMathLibrary.BreakVector` (`SplineComponent.GetLocationAtSplinePoint` _spline (`self.TargetFloor`) "Local")))
  (bind (_returnvalue_x_2 _returnvalue_y_2 _returnvalue_z_2) (`KismetMathLibrary.BreakVector` (`SplineComponent.GetLocationAtSplinePoint` _spline_2 (`self.TargetFloor`) "Local")))
  (:`Pressed`
    (bind _output_get (set `self.TargetFloor` 0))
    (`/Engine/EditorBlueprintResources/StandardMacros.CompareInt` _output_get (`self.CurrentFloor`)
      (:`>`
        (`TimelineComponent.SetPlayRate` _timeline_0 _speed :!label _label)
        (bind (_direction _newtrack_1) (`Timeline|Timeline_0` :!label _label_2)
          (:`Update`
            (switch `ETimelineDirection` _direction
              (:`Forward`
                (bind (_returnvalue_x_3 _returnvalue_y_3 _returnvalue_z_3) (`KismetMathLibrary.BreakVector` (`SplineComponent.GetLocationAtTime` _spline_2 _newtrack_1 "Local" false)))
                (if (< _returnvalue_z_3 _returnvalue_z_2)
                  (`SceneComponent.K2_SetRelativeLocation` (`self.Elevator`) (`KismetMathLibrary.MakeVector` 0.0 0.0 _returnvalue_z_3) false false)
                  (else
                    (set `self.CurrentFloor` (`self.TargetFloor`))
                    (goto _label_2 :!via `Stop`))))
              (:`Backward`
                (bind (_returnvalue_x_4 _returnvalue_y_4 _returnvalue_z_4) (`KismetMathLibrary.BreakVector` (`SplineComponent.GetLocationAtTime` _spline _newtrack_1 "Local" false)))
                (if (> _returnvalue_z_4 _returnvalue_z)
                  (`SceneComponent.K2_SetRelativeLocation` (`self.Elevator`) (`KismetMathLibrary.MakeVector` 0.0 0.0 _returnvalue_z_4) false false)
                  (else
                    (set `self.CurrentFloor` (`self.TargetFloor`))
                    (goto _label_2 :!via `Stop`))))))))
      (:`<`
        (`TimelineComponent.SetPlayRate` _timeline_0 _speed :!label _label_3)
        (goto _label_2 :!via `Reverse`)))))

(event `Key|Two`
  (params (Key :type "Key Structure"))
  (:`Pressed`
    (bind _output_get (set `self.TargetFloor` 1))
    (`/Engine/EditorBlueprintResources/StandardMacros.CompareInt` _output_get (`self.CurrentFloor`)
      (:`>`
        (goto _label))
      (:`<`
        (goto _label_3)))))

(event `Key|Three`
  (params (Key :type "Key Structure"))
  (:`Pressed`
    (bind _output_get (set `self.TargetFloor` 2))
    (`/Engine/EditorBlueprintResources/StandardMacros.CompareInt` _output_get (`self.CurrentFloor`)
      (:`>`
        (goto _label))
      (:`<`
        (goto _label_3)))))

(event `self.Box.OnComponentBeginOverlap`
  (params (OverlappedComponent :type "PrimitiveComponent Object Reference") (OtherActor :type "Actor Object Reference") (OtherComp :type "PrimitiveComponent Object Reference") (OtherBodyIndex :type Integer) (bFromSweep :type Boolean) (SweepResult :type "HitResult Structure (by ref)"))
  (cast `Pawn` OtherActor)
  (`self.EnableInput` (`GameplayStatics.GetPlayerController` 0)))

(fn `UserConstructionScript`)
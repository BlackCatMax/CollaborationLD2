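; BP_Door is an interactable door that the ALS player character opens and closes with Interact, optionally requiring a key.
; Overlapping its Sphere enables input and opens a Gate; leaving disables both, as does BeginPlay.
; With NeedKey set, the character's HasKey is consumed to unlock it permanently, otherwise a WB_NeedKey widget appears.
; A FlipFlop alternately plays and reverses the OpenClose timeline that drives the mesh's yaw.
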(event `InputAction|Interact`
  (params (Key :type "Key Structure"))
  (:`Pressed`
    (if (`self.Need Key?`)
      (if (`/Game/AdvancedLocomotionV4/Blueprints/CharacterLogic/ALS_AnimMan_CharacterBP.HasKey?` (stale `self.Sphere.OnComponentBeginOverlap` _asals_anim_man_character_bp))
        (`|ExecutionSequence`
          (:`then_0`
            (`/Engine/EditorBlueprintResources/StandardMacros.Gate` true :!label _label
              (:`Exit`
                (`/Engine/EditorBlueprintResources/StandardMacros.FlipFlop`
                  (:`A`
                    (bind (_direction _open_close) (`Timeline|Open-Close` :!label _label_2)
                      (:`Update`
                        (`SceneComponent.K2_SetRelativeLocationAndRotation` (`self.SM_Door`) (15.0 4.5 0.0) (`KismetMathLibrary.MakeRotator` 0.0 0.0 _open_close) false false))))
                  (:`B`
                    (goto _label_2 :!via `Reverse`))))))
          (:`then_1`
            (`/Engine/EditorBlueprintResources/StandardMacros.DoOnce` false
              (:`Completed`
                (set `self.Need Key?` false)
                (set `/Game/AdvancedLocomotionV4/Blueprints/CharacterLogic/ALS_AnimMan_CharacterBP.HasKey?` false (stale `self.Sphere.OnComponentBeginOverlap` _asals_anim_man_character_bp))))))
        (else
          (bind _returnvalue (`|CreateWidget` "/Game/UI/WB_NeedKey.WB_NeedKey_C"))
          (`UserWidget.AddToViewport` _returnvalue 0)))
      (else
        (goto _label)))))

(event `self.Sphere.OnComponentBeginOverlap`
  (params (OverlappedComponent :type "PrimitiveComponent Object Reference") (OtherActor :type "Actor Object Reference") (OtherComp :type "PrimitiveComponent Object Reference") (OtherBodyIndex :type Integer) (bFromSweep :type Boolean) (SweepResult :type "HitResult Structure (by ref)"))
  (bind _asals_anim_man_character_bp (cast `/Game/AdvancedLocomotionV4/Blueprints/CharacterLogic/ALS_AnimMan_CharacterBP` OtherActor))
  (`self.EnableInput` (`GameplayStatics.GetPlayerController` 0))
  (goto _label :!via `Open`))

(event `self.Sphere.OnComponentEndOverlap`
  (params (OverlappedComponent :type "PrimitiveComponent Object Reference") (OtherActor :type "Actor Object Reference") (OtherComp :type "PrimitiveComponent Object Reference") (OtherBodyIndex :type Integer))
  (cast `/Game/AdvancedLocomotionV4/Blueprints/CharacterLogic/ALS_AnimMan_CharacterBP` OtherActor)
  (`self.DisableInput` (`GameplayStatics.GetPlayerController` 0) :!label _label_3)
  (goto _label :!via `Close`))

(event `self.ReceiveBeginPlay`
  (goto _label_3))

(fn `UserConstructionScript`)